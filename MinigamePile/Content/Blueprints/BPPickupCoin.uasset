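; Coin pickup for the rolling minigame that counts toward completing the level.
; It overrides the parent's IncreaseScore to increment the pickups collected this level in the game instance and compare it to the game mode's required count.
; At the threshold, it activates the first OpenLevelLoadWidgetWithPrompt actor and calls its overlap handler with the first default-pawn-class actor, so no travel to that actor is needed.
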(event `self.ReceiveBeginPlay`
  (`parent.ReceiveBeginPlay`)
  (bind _asminigame_pile_game_instance (cast `/Game/Blueprints/MinigamePileGameInstance` (`GameplayStatics.GetGameInstance`)))
  (set `self.GameInstanceRef` _asminigame_pile_game_instance)
  (bind _asrolling_game_mode (cast `/Game/GameModes/RollingGameMode` (`GameplayStatics.GetGameMode`)))
  (set `self.RollGameModeRef` _asrolling_game_mode))

(event `self.IncreaseScore`
  (bind _rollgamemoderef (`self.RollGameModeRef`))
  ;[1 1 1] override 'increase score' to be increment pickups collected
  (bind _result (`/Engine/EditorBlueprintResources/StandardMacros.IncrementInt` (`/Game/Blueprints/MinigamePileGameInstance.PickupsCollectedThisLevel` (`self.GameInstanceRef`)))
    (:`  `
      (if (>= _result (`/Game/GameModes/RollingGameMode.PickupsRequiredToAdvance` _rollgamemoderef))
        (bind _outactors (`GameplayStatics.GetAllActorsOfClass` (`GameModeBase.DefaultPawnClass` _rollgamemoderef)))
        (bind _outactors_2 (`GameplayStatics.GetAllActorsOfClass` "/Game/Blueprints/OpenLevelLoadWidgetWithPrompt.OpenLevelLoadWidgetWithPrompt_C"))
        (bind _output (`|GetArrayItem` _outactors_2))
        (set `/Game/Blueprints/OpenLevelLoadWidgetWithPrompt.Activated` true _output)
        ;;[1 0.6854 0.184] dont call if we decide to require travel to actor. could instead set hud message t osay "get to the finish point!"
        (`/Game/Blueprints/OpenLevelLoadWidgetWithPrompt.HandleBeginOverlap` _output (`|GetArrayItem` _outactors))))))

(fn `UserConstructionScript`
  (`parent.UserConstructionScript`))