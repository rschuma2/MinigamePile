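; Trigger volume that shows a PlaySimoneQuestionWidget prompt while the ThirdPersonCharacter stands inside its Box.
; On begin overlap it creates the widget once, caches it for reuse, adds it to the viewport, shows the mouse cursor and switches to Game and UI input focused on it.
; On end overlap it removes the widget, hides the cursor and restores game-only input.
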(event `self.Box.OnComponentBeginOverlap`
  (params (OverlappedComponent :type "PrimitiveComponent Object Reference") (OtherActor :type "Actor Object Reference") (OtherComp :type "PrimitiveComponent Object Reference") (OtherBodyIndex :type Integer) (bFromSweep :type Boolean) (SweepResult :type "HitResult Structure (by ref)"))
  (bind _returnvalue (`GameplayStatics.GetPlayerController` 0))
  (bind _widget (`self.Widget`))
  (cast `/Game/Characters/ThirdPersonCharacter` OtherActor)
  (`/Engine/EditorBlueprintResources/StandardMacros.IsValid` (`self.Widget`)
    (:`Is Valid`
      (if (not (`Widget.IsInViewport` _widget))
        (`UserWidget.AddToViewport` (stale _returnvalue_2) 0 :!label _label)
        (`UserWidget.AddToViewport` (stale _output_get) 0)
        (`UserWidget.AddToViewport` _widget 0)
        (set `PlayerController.bShowMouseCursor` true _returnvalue)
        (`WidgetBlueprintLibrary.SetInputMode_GameAndUIEx` _returnvalue _widget)))
    (:`Is Not Valid`
      (bind _returnvalue_2 (`|CreateWidget` "/Game/widgets/Simone/PlaySimoneQuestionWidget.PlaySimoneQuestionWidget_C" _returnvalue))
      (bind _output_get (set `self.Widget` _returnvalue_2))
      (goto _label))))

(event `self.Box.OnComponentEndOverlap`
  (params (OverlappedComponent :type "PrimitiveComponent Object Reference") (OtherActor :type "Actor Object Reference") (OtherComp :type "PrimitiveComponent Object Reference") (OtherBodyIndex :type Integer))
  (bind _returnvalue (`GameplayStatics.GetPlayerController` 0))
  (cast `/Game/Characters/ThirdPersonCharacter` OtherActor)
  (`Widget.RemoveFromParent` (`self.Widget`))
  (set `PlayerController.bShowMouseCursor` false _returnvalue)
  (`WidgetBlueprintLibrary.SetInputMode_GameOnly` _returnvalue))

(fn `UserConstructionScript`)