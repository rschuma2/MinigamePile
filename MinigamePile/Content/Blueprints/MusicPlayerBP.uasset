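; Music player Blueprint that starts a music track with a fade-in when play begins.
; On BeginPlay it picks either a random entry from its variant array or the single default track, depending on a variants flag.
; The choice goes to the PlayMusic event, which sets the sound on the Music audio component and fades it in to partial volume.
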(event `PlayMusic`
  (params (NewSound :type "SoundBase Object Reference"))
  (bind _music (`self.Music`))
  ;[1 1 1] Play Music
  (`AudioComponent.SetSound` _music NewSound)
  (`AudioComponent.FadeIn` _music 3.0 0.5 0.0))

(event `self.ReceiveBeginPlay`
  (if (`self.HasVariants`)
    (`self.PlayMusic` (`|GetArrayItem` (`self.MusicVariantArray`) (`KismetMathLibrary.RandomIntegerInRange` 0 (- (`self.NumSongVariants`) 1))))
    (else
      (`self.PlayMusic` (`self.MusicToPlay`)))))

(fn `UserConstructionScript`)