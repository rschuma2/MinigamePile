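; Player controller for the MinigamePile game that handles the pause and menu-focus inputs.
; Pause, if not already paused, pauses the game and opens a PauseScreen widget with UI-only input and a visible cursor; unpausing is not handled here.
; FocusMenu, gated by a GameInstance flag, focuses the play-game question widget and tries to freeze the character by disabling input and movement, which an inline comment reports as unreliable.
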(event `self.ReceiveBeginPlay`
  (bind _asminigame_pile_game_instance (cast `/Game/Blueprints/MinigamePileGameInstance` (`GameplayStatics.GetGameInstance`)))
  (set `self.GameInstanceRef` _asminigame_pile_game_instance))

(event `InputAction|Pause`
  (params (Key :type "Key Structure"))
  (bind _returnvalue (`GameplayStatics.GetPlayerController` 0))
  (:`Pressed`
    (if (not (`self.Paused`))
      (bind _returnvalue_2 (`GameplayStatics.SetGamePaused` true))
      (set `self.Paused` _returnvalue_2)
      (bind _returnvalue_3 (`|CreateWidget` "/Game/widgets/PauseScreen.PauseScreen_C"))
      (bind _output_get (set `self.PauseScreen` _returnvalue_3))
      (`UserWidget.AddToViewport` _returnvalue_3 0)
      (`UserWidget.AddToViewport` _output_get 0)
      (`WidgetBlueprintLibrary.SetInputMode_UIOnlyEx` _returnvalue _output_get)
      (set `PlayerController.bShowMouseCursor` true _returnvalue))))

(event `InputAction|FocusMenu`
  (params (Key :type "Key Structure"))
  (bind _returnvalue (`GameplayStatics.GetPlayerCharacter` 0))
  (bind _gameinstanceref (`self.GameInstanceRef`))
  (:`Pressed`
    (if (`/Game/Blueprints/MinigamePileGameInstance.LookForFocusAction` _gameinstanceref)
      (`/Game/widgets/Simone/PlayInsertGameQuestionWidget.FocusThisWidget` (`/Game/Blueprints/MinigamePileGameInstance.PlayGameQuestionWidget` _gameinstanceref))
      ;[1 1 1] This will never work. it is impossible to make a character stop moving normally when you pull up a widget. change my mind. affects playerinsert game question and open play game trigger and minigame pile player controller and my soul.
      (`self.DisableInput` _returnvalue (`GameplayStatics.GetPlayerController` 0))
      (`CharacterMovementComponent.SetMovementMode` (`Character.CharacterMovement` _returnvalue) "MOVE_None" 0))))

(fn `UserConstructionScript`)