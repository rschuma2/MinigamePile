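; CharSwapTrigger is a trigger actor that swaps the player's character when a ThirdPersonCharacter overlaps its Box.
; The overlap passes the SwapToClass variable to SwapCharacter, which destroys the pawn controlled by player controller 0.
; It then spawns the new class at the trigger's root location, not the old pawn's, and possesses it with that controller.
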(event `SwapCharacter`
  (params (SwapToClass :type "Pawn Class Reference"))
  (bind _returnvalue (`GameplayStatics.GetPlayerController` 0))
  (bind _returnvalue_2 (`Controller.K2_GetPawn` _returnvalue))
  (`/Engine/EditorBlueprintResources/StandardMacros.IsValid` _returnvalue_2
    (:`Is Valid`
      (`self.K2_DestroyActor` _returnvalue_2))
    (:`Is Not Valid`
      _))
  (bind _returnvalue_3 (`|SpawnActorFromClass` SwapToClass (`KismetMathLibrary.MakeTransform` (`SceneComponent.K2_GetComponentLocation` (`self.DefaultSceneRoot`))) "Undefined" "OverrideRootScale" null null))
  (`Controller.Possess` _returnvalue _returnvalue_3))

(event `self.Box.OnComponentBeginOverlap`
  (params (OverlappedComponent :type "PrimitiveComponent Object Reference") (OtherActor :type "Actor Object Reference") (OtherComp :type "PrimitiveComponent Object Reference") (OtherBodyIndex :type Integer) (bFromSweep :type Boolean) (SweepResult :type "HitResult Structure (by ref)"))
  (cast `/Game/PlayerCharacters/ThirdPerson/ThirdPersonCharacter` OtherActor)
  (`self.SwapCharacter` (`self.SwapToClass`)))

(fn `UserConstructionScript`)