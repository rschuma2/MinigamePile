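; Target actor for the target practice minigame, which awards points when its Sphere is hit.
; A hit adds to the game instance's TargetPracticeScore, with smaller spheres worth more, then spawns an explosion and destroys the actor.
; A looping timer removes the target once the sphere drops below its initial height, and a short lifespan also limits how long it exists.
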(event `self.ReceiveBeginPlay`
  (`KismetSystemLibrary.K2_SetTimerDelegate` (delegate `DestroyTarget`) 0.25 true)
  (`self.SetLifeSpan` 2.5))

(event `DestroyTarget`
  (bind (_returnvalue_x _returnvalue_y _returnvalue_z) (`KismetMathLibrary.BreakVector` (`SceneComponent.K2_GetComponentLocation` (`self.Sphere`))))
  (if (< _returnvalue_z (.z (.location (`self.InitialTransform`))))
    (`self.K2_DestroyActor`)))

(event `self.Sphere.OnComponentHit`
  (params (HitComponent :type "PrimitiveComponent Object Reference") (OtherActor :type "Actor Object Reference") (OtherComp :type "PrimitiveComponent Object Reference") (NormalImpulse :type "Vector Structure") (Hit :type "HitResult Structure (by ref)"))
  (bind _returnvalue_x (`KismetMathLibrary.BreakVector` (`SceneComponent.K2_GetComponentScale` (`self.Sphere`))))
  ;[1 1 1] Handle Sphere hit. Increase score and destroy target
  (bind _asminigame_pile_game_instance (cast `/Game/Blueprints/MinigamePileGameInstance` (`GameplayStatics.GetGameInstance`)))
  (set `/Game/Blueprints/MinigamePileGameInstance.TargetPracticeScore` (+ (`/Game/Blueprints/MinigamePileGameInstance.TargetPracticeScore` _asminigame_pile_game_instance) (`KismetMathLibrary.FTrunc` (- 200.0 (* _returnvalue_x 100.0)))) _asminigame_pile_game_instance)
  (`GameplayStatics.SpawnEmitterAtLocation` "/Game/ParticleEffects/P_Explosion.P_Explosion" (`SceneComponent.K2_GetComponentLocation` (`self.Sphere`)))
  (`self.K2_DestroyActor`))

(fn `UserConstructionScript`)