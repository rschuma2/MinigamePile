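; SpawnRing is a target-practice spawner that launches a limited supply of Target actors and displays the remaining count on a text render.
; The count is randomised at BeginPlay unless the instance is customised.
; A looping one-second timer, gated by Activated, spawns each target at a random point in the collision box's bounds.
; Each target gets a size and material from a shared random index, another random InitialTransform, and an upward impulse.
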(event `self.ReceiveBeginPlay`
  (`KismetSystemLibrary.K2_SetTimerDelegate` (delegate `SpawnTarget`) 1.0 true)
  (if (`self.InstanceCustomized`)
    (`TextRenderComponent.K2_SetText` (`self.TextRender`) (`KismetTextLibrary.Conv_IntToText` (`self.NumTargets`)))
    (else
      (bind _output_get (set `self.NumTargets` (`KismetMathLibrary.RandomIntegerInRange` 7 15)))
      (`TextRenderComponent.K2_SetText` (`self.TextRender`) (`KismetTextLibrary.Conv_IntToText` _output_get)))))

(event `SpawnTarget`
  (bind _sizearray (`self.SizeArray`))
  (bind (_origin _boxextent) (`KismetSystemLibrary.GetComponentBounds` (`self.SpawnVolumeCollisionBox`)))
  (bind _returnvalue (`KismetMathLibrary.Conv_VectorToTransform` (`KismetMathLibrary.RandomPointInBoundingBox` _origin _boxextent)))
  (if (`self.Activated`)
    (if (> (`self.NumTargets`) 0)
      (bind _returnvalue_2 (`|SpawnActorFromClass` "/Game/Blueprints/TargetPractice/Target.Target_C" _returnvalue "Undefined" "OverrideRootScale" null "0.000000,0.000000,0.000000|0.000000,0.000000,0.000000|1.000000,1.000000,1.000000" null))
      (bind _output_get (set `self.SpawnedTarget` _returnvalue_2))
      (bind _result (`/Engine/EditorBlueprintResources/StandardMacros.DecrementInt` (`self.NumTargets`))
        (:`  `
          (`TextRenderComponent.K2_SetText` (`self.TextRender`) (`KismetTextLibrary.Conv_IntToText` _result))
          (bind _output_get_2 (set `self.RandInt` (`KismetMathLibrary.RandomIntegerInRange` 0 (- (`KismetArrayLibrary.Array_Length` _sizearray) 1))))
          (bind _sphere (`/Game/Blueprints/TargetPractice/Target.Sphere` _output_get))
          (bind _output (`|GetArrayItem` _sizearray _output_get_2))
          (`SceneComponent.SetWorldScale3D` _sphere (`KismetMathLibrary.MakeVector` _output _output _output))
          (switch `int` 0
            (:`Default`
              (`PrimitiveComponent.SetMaterial` _sphere 0 (`|GetArrayItem` (`self.SphereColor`) _output_get_2))
              (set `/Game/Blueprints/TargetPractice/Target.InitialTransform` _returnvalue _output_get)
              (`PrimitiveComponent.AddImpulse` (`/Game/Blueprints/TargetPractice/Target.Sphere` _output_get) (0.0 0.0 20000.0) "None" false))))))))

(fn `UserConstructionScript`)