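; Trigger volume that offers the player a minigame level to play when their third-person character walks into its box.
; On overlap it plays an activated or deactivated sound, passes activation state, question text and target level to the GameInstance, which shows the prompt widget.
; On exit it removes the prompt, fades the activated sound and restores game-only input and walking, a reset the author notes as unreliable.
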(event `self.ReceiveBeginPlay`
  (bind _asminigame_pile_game_instance (cast `/Game/Blueprints/MinigamePileGameInstance` (`GameplayStatics.GetGameInstance`)))
  (set `self.GameInstanceRef` _asminigame_pile_game_instance)
  (bind _returnvalue (`|CreateWidget` "/Game/widgets/PlayInsertGameQuestionWidget.PlayInsertGameQuestionWidget_C"))
  (set `self.ThisWidget` _returnvalue))

(event `self.Box.OnComponentBeginOverlap`
  (params (OverlappedComponent :type "PrimitiveComponent Object Reference") (OtherActor :type "Actor Object Reference") (OtherComp :type "PrimitiveComponent Object Reference") (OtherBodyIndex :type Integer) (bFromSweep :type Boolean) (SweepResult :type "HitResult Structure (by ref)"))
  (bind _gameinstanceref (`self.GameInstanceRef`))
  (cast `/Game/PlayerCharacters/ThirdPerson/ThirdPersonCharacter` OtherActor)
  (if (`self.Activated`)
    (`AudioComponent.Play` (`self.ActivatedSound`) 0.0)
    (else
      (`AudioComponent.Play` (`self.DeactivatedSound`) 0.0)))
  (set `/Game/Blueprints/MinigamePileGameInstance.WidgetActivated` (`self.Activated`) (`self.GameInstanceRef`))
  (set `/Game/Blueprints/MinigamePileGameInstance.PlayQuestionText` (`self.UpdateWidgetText`) _gameinstanceref)
  (set `/Game/Blueprints/MinigamePileGameInstance.LevelToOpen` (`self.LevelToOpen`) _gameinstanceref)
  (`/Game/Blueprints/MinigamePileGameInstance.ShowPlayGameQuestionWidget` (`self.GameInstanceRef`)))

(event `self.Box.OnComponentEndOverlap`
  (params (OverlappedComponent :type "PrimitiveComponent Object Reference") (OtherActor :type "Actor Object Reference") (OtherComp :type "PrimitiveComponent Object Reference") (OtherBodyIndex :type Integer))
  (bind _returnvalue (`GameplayStatics.GetPlayerCharacter` 0))
  (bind _returnvalue_2 (`GameplayStatics.GetPlayerController` 0))
  (bind _gameinstanceref (`self.GameInstanceRef`))
  (bind _playgamequestionwidget (`/Game/Blueprints/MinigamePileGameInstance.PlayGameQuestionWidget` _gameinstanceref))
  (cast `/Game/PlayerCharacters/ThirdPerson/ThirdPersonCharacter` OtherActor)
  (`Widget.RemoveFromParent` _playgamequestionwidget)
  (set `/Game/Blueprints/MinigamePileGameInstance.LookForFocusAction` false _gameinstanceref)
  (`Widget.SetVisibility` (`/Game/widgets/PlayInsertGameQuestionWidget.FToFocusOverlay` _playgamequestionwidget) "Visible")
  (`AudioComponent.FadeOut` (`self.ActivatedSound`) 0.5 0.0)
  ;[1 1 1] This will never work. it is impossible to make a character stop moving normally when you pull up a widget. change my mind. affects playerinsert game question and open play game trigger and minigame pile player controller and my soul.
  (`WidgetBlueprintLibrary.SetInputMode_GameOnly` _returnvalue_2)
  (set `PlayerController.bShowMouseCursor` false _returnvalue_2)
  (`CharacterMovementComponent.SetMovementMode` (`Character.CharacterMovement` _returnvalue) "MOVE_Walking" 0)
  (`self.EnableInput` _returnvalue _returnvalue_2))

(fn `UserConstructionScript`)