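; Level segment for an endless flying game that decorates itself, spawns pickups and keeps the track going.
; On BeginPlay it scatters terrain and left and right wall meshes within box volumes through a DoN loop.
; A looping timer spawns shuffled, limited-lifespan pickups at random points in their volume.
; FlyingPawn overlapping StartCollision spawns a segment ahead if SpawnNext is set; overlapping EndCollision destroys this one after a delay.
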(event `self.ReceiveBeginPlay`
  ;[1 1 1] Begin Play. Start timer to spawn pickups and spawn terrain/'wall' decorations
  (bind _returnvalue (`KismetSystemLibrary.K2_SetTimerDelegate` (delegate `HandlePickupSpawnTimer`) 2.0 true))
  (set `self.PickupSpawnTimerHandle` _returnvalue)
  (`self.SpawnStuff`))

(event `SpawnStuff`
  ;[1 1 1] Spawn Stuff!
  (`/Engine/EditorBlueprintResources/StandardMacros.Do N` 10 :!label _label
    (:`Exit`
      (`self.SpawnTerrain`)
      (`self.SpawnLeftWall`)
      (`self.SpawnRightWall`)
      (goto _label))))

(event `HandlePickupSpawnTimer`
  (bind _pickupspawnvolume (`self.PickupSpawnVolume`))
  (bind _pickuparray (`self.PickupArray`))
  ;[1 1 1] Spawn Pickups
  (`KismetArrayLibrary.Array_Shuffle` _pickuparray)
  (bind _returnvalue (`|SpawnActorFromClass` (`|GetArrayItem` _pickuparray) (`KismetMathLibrary.MakeTransform` (`KismetMathLibrary.RandomPointInBoundingBox` (`SceneComponent.K2_GetComponentLocation` _pickupspawnvolume) (`BoxComponent.GetScaledBoxExtent` _pickupspawnvolume))) "Undefined" "OverrideRootScale" null null))
  (`self.SetLifeSpan` _returnvalue 30.0))

(event `SpawnTerrain`
  (bind (_returnvalue_roll _returnvalue_pitch _returnvalue_yaw) (`KismetMathLibrary.BreakRotator` (`KismetMathLibrary.RandomRotator` false)))
  (bind _terrainspawnvolume (`self.TerrainSpawnVolume`))
  ;[1 1 1] Spawn Stuff!
  (`AddComponent|NODE_AddStaticMeshComponent-1` :`RelativeTransform` (`KismetMathLibrary.MakeTransform` (`KismetMathLibrary.RandomPointInBoundingBox` (`SceneComponent.RelativeLocation` _terrainspawnvolume) (`BoxComponent.GetScaledBoxExtent` _terrainspawnvolume)) (`KismetMathLibrary.MakeRotator` 0.0 0.0 _returnvalue_yaw))))

(event `self.StartCollision.OnComponentBeginOverlap`
  (params (OverlappedComponent :type "PrimitiveComponent Object Reference") (OtherActor :type "Actor Object Reference") (OtherComp :type "PrimitiveComponent Object Reference") (OtherBodyIndex :type Integer) (bFromSweep :type Boolean) (SweepResult :type "HitResult Structure (by ref)"))
  (bind (_returnvalue_x _returnvalue_y _returnvalue_z) (`KismetMathLibrary.BreakVector` (`SceneComponent.K2_GetComponentLocation` (`self.EndCollision`))))
  ;[1 1 1] Spawn next segment
  (cast `/Game/PlayerCharacters/Infiniflier/FlyingPawn` OtherActor)
  (if (`self.SpawnNext`)
    (`|SpawnActorFromClass` "SpawnSegments_C" (`KismetMathLibrary.MakeTransform` (`KismetMathLibrary.MakeVector` (+ _returnvalue_x (* (`self.SegmentsToSkip`) 1975.0)) _returnvalue_y _returnvalue_z)) "Undefined" "OverrideRootScale" null null)))

(event `SpawnLeftWall`
  (bind _leftwallspawnvolume (`self.LeftWallSpawnVolume`))
  ;[1 1 1] Spawn Stuff!
  (bind _returnvalue (`AddComponent|NODE_AddStaticMeshComponent-2` :`RelativeTransform` (`KismetMathLibrary.MakeTransform` (`KismetMathLibrary.RandomPointInBoundingBox` (`SceneComponent.RelativeLocation` _leftwallspawnvolume) (`BoxComponent.GetScaledBoxExtent` _leftwallspawnvolume))))))

(event `self.EndCollision.OnComponentBeginOverlap`
  (params (OverlappedComponent :type "PrimitiveComponent Object Reference") (OtherActor :type "Actor Object Reference") (OtherComp :type "PrimitiveComponent Object Reference") (OtherBodyIndex :type Integer) (bFromSweep :type Boolean) (SweepResult :type "HitResult Structure (by ref)"))
  ;[1 1 1] Destroy previous segment
  (cast `/Game/PlayerCharacters/Infiniflier/FlyingPawn` OtherActor)
  (`KismetSystemLibrary.Delay` 2.0)
  (`self.K2_DestroyActor`))

(event `SpawnRightWall`
  (bind _rightwallspawnvolume (`self.RightWallSpawnVolume`))
  ;[1 1 1] Spawn Stuff!
  (`AddComponent|NODE_AddStaticMeshComponent-3` :`RelativeTransform` (`KismetMathLibrary.MakeTransform` (`KismetMathLibrary.RandomPointInBoundingBox` (`SceneComponent.RelativeLocation` _rightwallspawnvolume) (`BoxComponent.GetScaledBoxExtent` _rightwallspawnvolume)) (struct))))

(fn `UserConstructionScript`)