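; Energy refill pickup Blueprint for Infiniflier that rewards the player on overlap and then removes itself.
; On BeginPlay it caches the player's controlled FlyingPawn.
; When an actor whose class is in the Characters list enters its sphere, a DoOnce adds Value to the GameMode score, plays a sound and calls IncreaseEnergy on the cached pawn.
; After a short delay the pickup destroys itself.
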(event `self.ReceiveBeginPlay`
  (`parent.ReceiveBeginPlay`)
  (bind _asflying_pawn (cast `/Game/PlayerCharacters/Infiniflier/FlyingPawn` (`Controller.K2_GetPawn` (`GameplayStatics.GetPlayerController` 0))))
  (set `self.PawnRef_0` _asflying_pawn))

(event `self.Sphere1.OnComponentBeginOverlap`
  (params (OverlappedComponent :type "PrimitiveComponent Object Reference") (OtherActor :type "Actor Object Reference") (OtherComp :type "PrimitiveComponent Object Reference") (OtherBodyIndex :type Integer) (bFromSweep :type Boolean) (SweepResult :type "HitResult Structure (by ref)"))
  (bind _gamemoderef (`self.GameModeRef`))
  (if (`BlueprintSetLibrary.Set_Contains` (`self.Characters`) (`GameplayStatics.GetObjectClass` OtherActor))
    (`/Engine/EditorBlueprintResources/StandardMacros.DoOnce` false
      (:`Completed`
        (set `/Game/GameModes/InfiniflierGameMode.Score` (+ (`/Game/GameModes/InfiniflierGameMode.Score` _gamemoderef) (`self.Value`)) _gamemoderef)
        (`GameplayStatics.PlaySound2D` "/Game/Audio/Music/Rhodesmas/380266__rhodesmas__alert-01.380266__rhodesmas__alert-01" 1.0 1.0 0.0 null null)
        (`/Game/PlayerCharacters/Infiniflier/FlyingPawn.IncreaseEnergy` (`self.PawnRef_0`))
        (`KismetSystemLibrary.Delay` 0.4)
        (`self.K2_DestroyActor`)))))

(fn `UserConstructionScript`
  (`parent.UserConstructionScript`))