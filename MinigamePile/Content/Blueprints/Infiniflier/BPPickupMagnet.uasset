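; Magnet pickup for Infiniflier that temporarily widens the reach of other pickups when an allowed character class overlaps it.
; On first overlap it enlarges the collision sphere of every "Pickup"-tagged BPPickupBase tenfold, with a delayed reset to normal scale.
; The actor destroys itself shortly after triggering, before that reset delay elapses.
; An unwired timeline lerp toward the player pawn remains unused.
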(event `self.ReceiveBeginPlay`
  (`parent.ReceiveBeginPlay`)
  (bind _asflying_pawn (cast `/Game/PlayerCharacters/Infiniflier/FlyingPawn` (`Controller.K2_GetPawn` (`GameplayStatics.GetPlayerController` 0))))
  (set `self.PawnRef_0` _asflying_pawn))

(event `GatherPickups`
  (bind _outactors (`GameplayStatics.GetAllActorsWithTag` "Pickup"))
  (bind _output_get (set `self.PickupArray` _outactors))
  (for _array_element _output_get
    (bind _asbppickup_base (cast `/Game/Blueprints/BPPickupBase` _array_element))
    (`SceneComponent.SetWorldScale3D` (`/Game/Blueprints/BPPickupBase.Sphere1` _asbppickup_base) (10.0 10.0 10.0)))
  (`KismetSystemLibrary.Delay` 3.0)
  (for _array_element_2 _output_get
    (bind _asbppickup_base_2 (cast `/Game/Blueprints/BPPickupBase` _array_element_2))
    (`SceneComponent.SetWorldScale3D` (`/Game/Blueprints/BPPickupBase.Sphere1` _asbppickup_base_2) (1.0 1.0 1.0)))
  (`KismetSystemLibrary.PrintString` "wowee"))

(event `self.Sphere1.OnComponentBeginOverlap`
  (params (OverlappedComponent :type "PrimitiveComponent Object Reference") (OtherActor :type "Actor Object Reference") (OtherComp :type "PrimitiveComponent Object Reference") (OtherBodyIndex :type Integer) (bFromSweep :type Boolean) (SweepResult :type "HitResult Structure (by ref)"))
  (if (`BlueprintSetLibrary.Set_Contains` (`self.Characters`) (`GameplayStatics.GetObjectClass` OtherActor))
    (`/Engine/EditorBlueprintResources/StandardMacros.DoOnce` false
      (:`Completed`
        (`self.GatherPickups`)
        (`KismetSystemLibrary.Delay` 0.4)
        (`self.K2_DestroyActor`)))))

(fn `UserConstructionScript`
  (`parent.UserConstructionScript`))