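; Boost refill pickup for the Infiniflier game that grants the player a boost and score when collected.
; A sphere overlap filters actors against a list of character classes and fires only once.
; It increments the pawn's available boosts, adds its value to the game mode score, plays a purchase sound, then destroys itself after a short delay.
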(event `self.ReceiveBeginPlay`
  (`parent.ReceiveBeginPlay`))

(event `self.Sphere1.OnComponentBeginOverlap`
  (params (OverlappedComponent :type "PrimitiveComponent Object Reference") (OtherActor :type "Actor Object Reference") (OtherComp :type "PrimitiveComponent Object Reference") (OtherBodyIndex :type Integer) (bFromSweep :type Boolean) (SweepResult :type "HitResult Structure (by ref)"))
  (bind _gamemoderef (`self.GameModeRef`))
  (if (`BlueprintSetLibrary.Set_Contains` (`self.Characters`) (`GameplayStatics.GetObjectClass` OtherActor))
    (`/Engine/EditorBlueprintResources/StandardMacros.DoOnce` false
      (:`Completed`
        (`/Engine/EditorBlueprintResources/StandardMacros.IncrementInt` (`/Game/PlayerCharacters/Infiniflier/FlyingPawn.BoostsAvailable` (`self.PawnRef`))
          (:`  `
            (set `/Game/GameModes/InfiniflierGameMode.Score` (+ (`/Game/GameModes/InfiniflierGameMode.Score` _gamemoderef) (`self.Value`)) _gamemoderef)
            (`GameplayStatics.PlaySound2D` "/Game/Audio/Music/Rhodesmas/342751__rhodesmas__coins-purchase-3.342751__rhodesmas__coins-purchase-3" 1.0 1.0 0.0 null null)
            (`KismetSystemLibrary.Delay` 0.4)
            (`self.K2_DestroyActor`)))))))

(fn `UserConstructionScript`
  (`parent.UserConstructionScript`))