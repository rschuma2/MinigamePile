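; Grid actor for a memory match game that spawns the blocks and checks whether two clicked ones match.
; On BeginPlay it shuffles the character material array, then lays out a Size-by-Size square of MemoryMatchBlocks from its location using modulo and division.
; Each block receives the grid as owner, its index and the next material, which is removed from the array.
; TestBlocksClicked compares the active materials of the first two BlocksClicked entries.
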(event `self.ReceiveBeginPlay`
  (bind _size (`self.Size`))
  (bind _charactermaterialarray (`self.CharacterMaterialArray`))
  (bind _size_2 (`self.Size`))
  (bind _blockspacing (`self.BlockSpacing`))
  ;[1 1 1] Spawn blocks
  (`KismetArrayLibrary.Array_Shuffle` (`self.CharacterMaterialArray`))
  (for _index (range (* _size _size))
    (bind _returnvalue (`|SpawnActorFromClass` "/Game/Blueprints/MemoryMatch/MemoryMatchBlock.MemoryMatchBlock_C" (`KismetMathLibrary.Conv_VectorToTransform` (+ (`KismetMathLibrary.MakeVector` (* (mod _index _size_2) _blockspacing) (* (/ _index _size_2) _blockspacing)) (`self.K2_GetActorLocation`))) "AlwaysSpawn" "OverrideRootScale" null self _index (`|GetArrayItem` _charactermaterialarray) null)) ; Spawn a  block
    (`KismetArrayLibrary.Array_Add` (`self.BlocksArray`) _returnvalue)
    (`KismetArrayLibrary.Array_Remove` _charactermaterialarray)))

(fn `TestBlocksClicked`
  (returns (BlocksMatch :type Boolean))
  (bind _blocksclicked (`self.BlocksClicked`))
  (return (== (`/Game/Blueprints/MemoryMatch/MemoryMatchBlock.BlockActiveMaterial` (`|GetArrayItem` _blocksclicked)) (`/Game/Blueprints/MemoryMatch/MemoryMatchBlock.BlockActiveMaterial` (`|GetArrayItem` _blocksclicked 1)))))

(fn `UserConstructionScript`)