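; Trigger volume that opens a level select widget when a character of an allowed class enters its box.
; On overlap begin it checks the actor's class against the Characters list, creates and shows the widget, and switches to Game and UI input with a visible cursor.
; On overlap end it removes the widget and restores game-only input with the cursor hidden.
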(event `self.Box.OnComponentBeginOverlap`
  (params (OverlappedComponent :type "PrimitiveComponent Object Reference") (OtherActor :type "Actor Object Reference") (OtherComp :type "PrimitiveComponent Object Reference") (OtherBodyIndex :type Integer) (bFromSweep :type Boolean) (SweepResult :type "HitResult Structure (by ref)"))
  (bind _returnvalue (`GameplayStatics.GetPlayerController` 0))
  (if (`BlueprintSetLibrary.Set_Contains` (`self.Characters`) (`GameplayStatics.GetObjectClass` OtherActor))
    (bind _returnvalue_2 (`|CreateWidget` "/Game/widgets/LevelSelectWidget.LevelSelectWidget_C"))
    (bind _output_get (set `self.LevelSelectWidget` _returnvalue_2))
    (`UserWidget.AddToViewport` _output_get 0)
    (`WidgetBlueprintLibrary.SetInputMode_GameAndUIEx` _returnvalue (`self.LevelSelectWidget`))
    (set `PlayerController.bShowMouseCursor` true _returnvalue)))

(event `self.Box.OnComponentEndOverlap`
  (params (OverlappedComponent :type "PrimitiveComponent Object Reference") (OtherActor :type "Actor Object Reference") (OtherComp :type "PrimitiveComponent Object Reference") (OtherBodyIndex :type Integer))
  (bind _returnvalue (`GameplayStatics.GetPlayerController` 0))
  (if (`BlueprintSetLibrary.Set_Contains` (`self.Characters`) (`GameplayStatics.GetObjectClass` OtherActor))
    (`Widget.RemoveFromParent` (`self.LevelSelectWidget`))
    (`WidgetBlueprintLibrary.SetInputMode_GameOnly` _returnvalue)
    (set `PlayerController.bShowMouseCursor` false _returnvalue)))

(fn `UserConstructionScript`)