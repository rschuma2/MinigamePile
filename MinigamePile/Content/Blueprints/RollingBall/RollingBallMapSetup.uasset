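; Per-map setup Blueprint for the rolling ball minigame that hands level settings to the game mode.
; On BeginPlay it caches the MinigamePile game instance and RollingGameMode, then after a short delay passes pickup requirement, pickup win condition, music and level to open via GetLevelSettings.
; An unset LevelToOpen falls back to the current level's name.
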(event `self.ReceiveBeginPlay`
  (`|ExecutionSequence`
    (:`then_0`
      (bind _asminigame_pile_game_instance (cast `/Game/Blueprints/MinigamePileGameInstance` (`GameplayStatics.GetGameInstance`)))
      (set `self.GameInstanceRef` _asminigame_pile_game_instance)
      (bind _asrolling_game_mode (cast `/Game/GameModes/RollingGameMode` (`GameplayStatics.GetGameMode`)))
      (set `self.GameModeRef` _asrolling_game_mode))
    (:`then_1`
      (`KismetSystemLibrary.Delay` 0.2)
      (if (== (`self.LevelToOpen`) "None")
        (bind _returnvalue (`GameplayStatics.GetCurrentLevelName` true))
        (set `self.LevelToOpen` (`KismetStringLibrary.Conv_StringToName` _returnvalue)))
      (`/Game/GameModes/RollingGameMode.GetLevelSettings` (`self.GameModeRef`) (`self.PickupsRequiredToAdvance`) (`self.MusicToPlay`) (`self.PickupWinCondition`) (`self.LevelToOpen`)))))

(fn `UserConstructionScript`)