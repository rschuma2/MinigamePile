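; Floor kill obstacle for the rolling ball minigame that ends the game when a playable character touches its box.
; BeginPlay caches the player's PhysicsBallBP and the RollingGameMode.
; An overlap by any class in the game instance's Characters list spawns an explosion at the obstacle and plays a sound.
; After a short delay it hides the cached ball and calls GameOver on the game mode.
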(event `self.ReceiveBeginPlay`
  (bind _asphysics_ball_bp (cast `/Game/PlayerCharacters/RollerBall/PhysicsBallBP` (`Controller.K2_GetPawn` (`GameplayStatics.GetPlayerController` 0))))
  (set `self.BallRef` _asphysics_ball_bp)
  (bind _asrolling_game_mode (cast `/Game/GameModes/RollingGameMode` (`GameplayStatics.GetGameMode`)))
  (set `self.GameModeRef` _asrolling_game_mode))

(event `self.Box.OnComponentBeginOverlap`
  (params (OverlappedComponent :type "PrimitiveComponent Object Reference") (OtherActor :type "Actor Object Reference") (OtherComp :type "PrimitiveComponent Object Reference") (OtherBodyIndex :type Integer) (bFromSweep :type Boolean) (SweepResult :type "HitResult Structure (by ref)"))
  (if (`KismetArrayLibrary.Array_Contains` (`/Game/Blueprints/MinigamePileGameInstance.Characters` (cast `/Game/Blueprints/MinigamePileGameInstance` (`GameplayStatics.GetGameInstance`) :!pure true)) (`GameplayStatics.GetObjectClass` OtherActor))
    (`GameplayStatics.SpawnEmitterAtLocation` "/Game/ParticleEffects/P_Explosion.P_Explosion" (`self.K2_GetActorLocation`))
    (`GameplayStatics.PlaySound2D` "/Game/Audio/Bluezone_BC0244_explosion_009_01.Bluezone_BC0244_explosion_009_01" 3.0 1.0 0.0 null null)
    (`KismetSystemLibrary.Delay` 0.2)
    (`self.SetActorHiddenInGame` (`self.BallRef`) true)
    (`/Game/GameModes/RollingGameMode.GameOver` (`self.GameModeRef`))))

(fn `UserConstructionScript`)