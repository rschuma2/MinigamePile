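; A HUD Blueprint that shows the EasyDriver pawn's speed and gear as on-screen text.
; Each DrawHUD pass casts the owning pawn to EasyDriver and draws only while its IsInCar flag is false.
; It computes scale ratios against a 720p baseline to position and size the text at any resolution.
; The pawn supplies both display strings, and its reverse-gear flag picks the gear text colour.
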(event `self.ReceiveDrawHUD`
  (params (SizeX :type Integer) (SizeY :type Integer))
  (bind _hudyratio (`self.HUDYRatio`))
  (bind _hudyratio_2 (`self.HUDYRatio`))
  ;[1 1 1] Calculate ratio from 720p
  (bind _aseasy_driver (cast `/Game/PlayerCharacters/EasyDriver/EasyDriver` (`self.GetOwningPawn`)))
  (if (not (`/Game/PlayerCharacters/EasyDriver/EasyDriver.IsInCar` _aseasy_driver))
    (`|ExecutionSequence`
      (:`then_0`
        (set `self.HUDXRatio` (/ (`KismetMathLibrary.Conv_IntToDouble` SizeX) 1280.0)))
      (:`then_1`
        (set `self.HUDYRatio` (/ (`KismetMathLibrary.Conv_IntToDouble` SizeY) 720.0)))
      (:`then_2`
        ;[1 1 1] Print vehicle speed
        (bind _aseasy_driver_2 (cast `/Game/PlayerCharacters/EasyDriver/EasyDriver` (`self.GetOwningPawn`)))
        (`self.DrawText` (`/Game/PlayerCharacters/EasyDriver/EasyDriver.Speed Display String` _aseasy_driver_2) (struct :`R` 1.0 :`G` 1.0 :`B` 1.0 :`A` 1.0) (* 805.0 (`self.HUDXRatio`)) (* 455.0 _hudyratio_2) "/Engine/EngineFonts/RobotoDistanceField.RobotoDistanceField" (* 1.4 _hudyratio_2))
        ;[1 1 1] Print vehicle gear
        (bind _aseasy_driver_3 (cast `/Game/PlayerCharacters/EasyDriver/EasyDriver` (`self.GetOwningPawn`)))
        (`self.DrawText` (`KismetStringLibrary.Concat_StrStr` "Gear:" (`/Game/PlayerCharacters/EasyDriver/EasyDriver.Gear Display String` _aseasy_driver_3)) (`KismetMathLibrary.SelectColor` (`/Game/PlayerCharacters/EasyDriver/EasyDriver.GearDisplayReverseColor` _aseasy_driver_3) (`/Game/PlayerCharacters/EasyDriver/EasyDriver.GearDisplayColor` _aseasy_driver_3) (`/Game/PlayerCharacters/EasyDriver/EasyDriver.InReverseGear` _aseasy_driver_3)) (* 805.0 (`self.HUDXRatio`)) (* 500.0 _hudyratio) "/Engine/EngineFonts/RobotoDistanceField.RobotoDistanceField" (* 1.4 _hudyratio)) ; If True display Current Gear
      ))))

(fn `UserConstructionScript`)